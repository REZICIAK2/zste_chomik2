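; Enemy room actor with a spider web that runs a two-spider wave and can be destroyed once the spiders are gone.
; StartWave picks random navmesh points around a hard-coded origin, plays spawn effects, then spawns spiders attached to itself.
; The attached-actor count tracks living enemies: at zero, Tick outlines the web through a DoOnce re-armed by StartWave.
; Player melee or projectile damage then destroys the actor.
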(event Custom|StartWave
  (Utilities|FlowControl|Sequence
    (:then_0
      (bind _randomlocation (Class|NavigationSystemV1|GetRandomLocationinNavigableRadius (Math|Vector|MakeVector 874.0 429.0 2619.0) 4e+02 0 0))
      (Game|SpawnActorfromClass "/Game/VFX/BP_SpawnEffect.BP_SpawnEffect_C" (Math|Transform|MakeTransform _randomlocation "0, 0, 0" "1.000000,1.000000,1.000000") "AdjustIfPossibleButAlwaysSpawn" "MultiplyWithRoot" 0 0)
      (Utilities|FlowControl|Delay 0.4)
      (bind _returnvalue (Game|SpawnActorfromClass "/Game/Enemies/Spiders/Spider/Blueprints/BP_Spider.BP_Spider_C" (Math|Conversions|ToTransform(Vector) _randomlocation) "Undefined" "MultiplyWithRoot" 0 0))
      (Transformation|AttachActorToActor _returnvalue self "None" "KeepWorld" "KeepWorld" "KeepWorld" true)
      (Utilities|FlowControl|DoOnce true) ; enters at Reset
    )
    (:then_1
      (bind _randomlocation_2 (Class|NavigationSystemV1|GetRandomLocationinNavigableRadius (Math|Vector|MakeVector 874.0 429.0 2619.0) 5e+02 0 0))
      (Game|SpawnActorfromClass "/Game/VFX/BP_SpawnEffect.BP_SpawnEffect_C" (Math|Transform|MakeTransform _randomlocation_2 "0, 0, 0" "1.000000,1.000000,1.000000") "AdjustIfPossibleButAlwaysSpawn" "MultiplyWithRoot" 0 0)
      (Utilities|FlowControl|Delay 0.4)
      (bind _returnvalue_2 (Game|SpawnActorfromClass "/Game/Enemies/Spiders/Spider/Blueprints/BP_Spider.BP_Spider_C" (Math|Conversions|ToTransform(Vector) _randomlocation_2) "Undefined" "MultiplyWithRoot" 0 0))
      (Transformation|AttachActorToActor _returnvalue_2 self "None" "KeepWorld" "KeepWorld" "KeepWorld" true))))

(event EventTick
  (params (DeltaSeconds :type Float%20%28single-precision%29))
  (if (== (Utilities|Array|Length (Actor|GetAttachedActors true false)) 0)
    (Utilities|FlowControl|DoOnce true
      (:Completed
        (Rendering|Material|SetMaterial (Variables|Default|Getspider_web) 0 "/Game/Materials/Materiały/OutlineMaterial.OutlineMaterial")))))

(event Game|Damage|EventAnyDamage
  (params (Damage :type Float%20%28single-precision%29) (DamageType :type Damage%20Type%20Object%20Reference) (InstigatedBy :type Controller%20Object%20Reference) (DamageCauser :type Actor%20Object%20Reference))
  (Utilities|Casting|CastToBP_PlayerAttackMelee DamageType
    (:then
      _)
    (:CastFailed
      (Utilities|Casting|CastToBP_PlayerAttackProjectail DamageType)))
  (if (== (Utilities|Array|Length (Actor|GetAttachedActors true false)) 0)
    (Actor|DestroyActor)))

(fn ConstructionScript)