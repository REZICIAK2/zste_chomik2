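; Cube enemy that melee-attacks the player and destroys itself when its health runs out.
; PawnSensing sighting triggers a forward sphere trace that damages the third-person character, then starts a cooldown.
; AnyDamage accepts only player melee and projectile damage types, while Tick updates a health bar widget turned toward the camera.
; Tick calls CalculateOffset for stalking, but that event is empty and the turn-and-chase movement logic is disconnected.
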(event OnSeePawn(PawnSensing)
  (params (Pawn :type Pawn%20Object%20Reference))
  ;[0.15 0.15 0.15 0.5] Combat system
  (Utilities|Casting|CastToBP_ThirdPersonCharacter Pawn)
  (if (Variables|Default|GetcanAttack)
    (CallFunction|AttackPlayer)))

(event Custom|Calculate%20Offset
  ;[0.15 0.15 0.15 0.5] Stalk player
)

(event Custom|Attack%20Player
  (bind _returnvalue (Transformation|GetActorLocation))
  (bind _returnvalue_2 (Transformation|GetActorRotation))
  (bind _returnvalue_3 (Math|Vector|GetForwardVector _returnvalue_2))
  (bind _returnvalue_4 (+ _returnvalue "0.000000,0.000000,100.000000"))
  ;[0.15 0.15 0.15 0.5] Combat system
  (bind (_outhit _returnvalue_5) (Collision|SphereTraceForObjects (+ (* _returnvalue_3 8e+01) _returnvalue_4) (+ _returnvalue_4 (* _returnvalue_3 1.7e+02)) 7e+01 (Utilities|Array|MakeArray "ObjectTypeQuery3") false 0 "None"))
  (if _returnvalue_5
    (Utilities|Casting|CastToBP_ThirdPersonCharacter (.HitActor (Collision|BreakHitResult _outhit)))
    (Game|Damage|ApplyDamage (.HitActor (Collision|BreakHitResult _outhit)) (Variables|Default|GetEnemy%20Demage) 0 0 "/Game/Blueprinty_silnika/BP_EnemyAttack.BP_EnemyAttack_C")
    (Variables|Default|SetcanAttack false)
    (Utilities|FlowControl|Delay 2.0)
    (Variables|Default|SetcanAttack true)))

(event Game|Damage|EventAnyDamage
  (params (Damage :type Float%20%28single-precision%29) (DamageType :type Damage%20Type%20Object%20Reference) (InstigatedBy :type Controller%20Object%20Reference) (DamageCauser :type Actor%20Object%20Reference))
  ;[0.15 0.15 0.15 0.5] Getting hit
  (Utilities|Casting|CastToBP_PlayerAttackMelee DamageType
    (:then
      _)
    (:CastFailed
      (Utilities|Casting|CastToBP_PlayerAttackProjectail DamageType)))
  (Variables|Default|SetHp (- (Variables|Default|GetHp) Damage)))

(event EventTick
  (params (DeltaSeconds :type Float%20%28single-precision%29))
  (bind _healthbar (Variables|Default|GetHealthBar))
  ;[0.15 0.15 0.15 0.5] Event tick
  (if (> (Variables|Default|GetHp) 0.0)
    (CallFunction|CalculateOffset)
    (bind _aswb_health_bar (Utilities|Casting|CastToWB_HealthBar (UserInterface|GetWidget (Variables|Default|GetHealthBar))))
    (Progress|SetPercent (Variables|/Game/Characters/WB_HealthBar.WB_HealthBar_C|GetHpBar _aswb_health_bar) (/ (Variables|Default|GetHp) 1e+02))
    (Transformation|SetWorldRotation _healthbar (Math|Rotator|FindLookatRotation (Transformation|GetWorldLocation _healthbar) (Transformation|GetWorldLocation (Variables|/Script/Engine.PlayerCameraManager|GetTransformComponent (Game|GetPlayerCameraManager 0)))) false false)
    (else
      (Actor|DestroyActor))))

(fn ConstructionScript)