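; BP_DefaultEnemy is an enemy that roams the navmesh and chases the player when they come within range.
; Sphere overlaps with BP_ThirdPersonCharacter toggle PlayerInRange and re-enter the shared StalkPlayer/StartRoam logic.
; That logic runs AI MoveTo at RunSpeed toward the player, or at WalkSpeed toward a random point within RoamRadius.
; Chase success or failure restarts the loop, while roaming restarts only on success.
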(event OnComponentBeginOverlap(Sphere)
  (params (OverlappedComponent :type Primitive%20Component%20Object%20Reference) (OtherActor :type Actor%20Object%20Reference) (OtherComp :type Primitive%20Component%20Object%20Reference) (OtherBodyIndex :type Integer) (bFromSweep :type Boolean) (SweepResult :type Hit%20Result%20Structure%20%28by%20ref%29))
  ;[0.15 0.15 0.15 0.5] Player in bot range
  (Utilities|Casting|CastToBP_ThirdPersonCharacter OtherActor)
  (Variables|Default|SetPlayerInRange true)
  (CallFunction|StalkPlayer))

(event OnComponentEndOverlap(Sphere)
  (params (OverlappedComponent :type Primitive%20Component%20Object%20Reference) (OtherActor :type Actor%20Object%20Reference) (OtherComp :type Primitive%20Component%20Object%20Reference) (OtherBodyIndex :type Integer))
  ;[0.15 0.15 0.15 0.5] Player in bot range
  (Utilities|Casting|CastToBP_ThirdPersonCharacter OtherActor)
  (Variables|Default|SetPlayerInRange false)
  (CallFunction|StalkPlayer))

(event Custom|Stalk%20Player
  (bind _self self)
  (bind _charactermovement (Variables|Character|GetCharacterMovement))
  ;[0.15 0.15 0.15 0.5] Roaming and stalking player
  (if (Variables|Default|GetPlayerInRange)
    (Variables|/Script/Engine.CharacterMovementComponent|SetMaxWalkSpeed _charactermovement (Variables|Default|GetRunSpeed))
    (AI|AIMoveTo _self "0, 0, 0" (Game|Player|GetPlayerPawn 0) 5.0 false
      (:OnSuccess
        _)
      (:OnFail
        _))
    (else
      (Variables|/Script/Engine.CharacterMovementComponent|SetMaxWalkSpeed _charactermovement (Variables|Default|GetWalkSpeed))
      (bind _randomlocation (Class|NavigationSystemV1|GetRandomLocationinNavigableRadius (Transformation|GetActorLocation) (Variables|Default|GetRoamRadius) 0 0))
      (AI|AIMoveTo _self _randomlocation 0 5.0 false
        (:OnSuccess
          _))))
  (CallFunction|StartRoam))

(event Custom|Start%20%20Roam
  (bind _self self)
  (bind _charactermovement (Variables|Character|GetCharacterMovement))
  ;[0.15 0.15 0.15 0.5] Roaming and stalking player
  (if (Variables|Default|GetPlayerInRange)
    (Variables|/Script/Engine.CharacterMovementComponent|SetMaxWalkSpeed _charactermovement (Variables|Default|GetRunSpeed))
    (AI|AIMoveTo _self "0, 0, 0" (Game|Player|GetPlayerPawn 0) 5.0 false
      (:OnSuccess
        _)
      (:OnFail
        _))
    (else
      (Variables|/Script/Engine.CharacterMovementComponent|SetMaxWalkSpeed _charactermovement (Variables|Default|GetWalkSpeed))
      (bind _randomlocation (Class|NavigationSystemV1|GetRandomLocationinNavigableRadius (Transformation|GetActorLocation) (Variables|Default|GetRoamRadius) 0 0))
      (AI|AIMoveTo _self _randomlocation 0 5.0 false
        (:OnSuccess
          _))))
  (CallFunction|StartRoam))

(event EventBeginPlay
  ;[0.15 0.15 0.15 0.5] Start
  (CallFunction|StartRoam))

(fn ConstructionScript)