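; Acid-spitting spider enemy that roams the navmesh and runs after the player while they overlap its detection sphere.
; Tick updates a camera-facing health bar, destroys the spider at zero HP, and calls Shoot while the player is detected.
; Within range, Shoot halts movement, plays the attack montage and spawns an acid projectile after a delay.
; Only the player's melee and projectile damage types reduce its HP.
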(event OnComponentBeginOverlap(Sphere)
  (params (OverlappedComponent :type Primitive%20Component%20Object%20Reference) (OtherActor :type Actor%20Object%20Reference) (OtherComp :type Primitive%20Component%20Object%20Reference) (OtherBodyIndex :type Integer) (bFromSweep :type Boolean) (SweepResult :type Hit%20Result%20Structure%20%28by%20ref%29))
  ;[0.15 0.15 0.15 0.5] Saw player
  (if (== OtherActor (Variables|Default|GetPlayerRef))
    (Variables|Default|SetSeePlayer? true)
    (CallFunction|StartRoam)))

(event OnComponentEndOverlap(Sphere)
  (params (OverlappedComponent :type Primitive%20Component%20Object%20Reference) (OtherActor :type Actor%20Object%20Reference) (OtherComp :type Primitive%20Component%20Object%20Reference) (OtherBodyIndex :type Integer))
  ;[0.15 0.15 0.15 0.5] Saw player
  (if (== (Variables|Default|GetPlayerRef) OtherActor)
    (Variables|Default|SetSeePlayer? false)
    (CallFunction|StartRoam)))

(event Custom|Start%20Roam
  (bind _self self)
  (bind _charactermovement (Variables|Character|GetCharacterMovement))
  ;[0.15 0.15 0.15 0.5] Roaming, and follow player
  (if (not (Variables|Default|GetAttacking?))
    (if (Variables|Default|GetSeePlayer?)
      (Variables|/Script/Engine.CharacterMovementComponent|SetMaxWalkSpeed _charactermovement (Variables|Default|GetRunSpeed))
      (AI|AIMoveTo _self "0, 0, 0" (Variables|Default|GetPlayerRef) 5.0 false
        (:OnSuccess
          _)
        (:OnFail
          _))
      (else
        (Variables|/Script/Engine.CharacterMovementComponent|SetMaxWalkSpeed _charactermovement (Variables|Default|GetWalkSpeed))
        (bind _randomlocation (Class|NavigationSystemV1|GetRandomLocationinNavigableRadius (Transformation|GetActorLocation) (Variables|Default|GetRoamRadius) 0 0))
        (AI|AIMoveTo _self _randomlocation 0 5.0 false
          (:OnSuccess
            _)
          (:OnFail
            _))))
    (CallFunction|StartRoam)))

(event Custom|Shoot
  (bind _playerref (Variables|Default|GetPlayerRef))
  ;[0.15 0.15 0.15 0.5] Attack
  (if (<= (Math|Vector|Distance(Vector) (Transformation|GetWorldLocation (Variables|/Script/Engine.Actor|GetRootComponent (Variables|Default|GetPlayerRef))) (Transformation|GetWorldLocation (Variables|Collision|GetCapsuleComponent))) 5e+02)
    (Variables|Default|SetAttacking? true)
    (if (Variables|Default|GetAttacking?)
      (Variables|/Script/Engine.CharacterMovementComponent|SetMaxWalkSpeed (Variables|Character|GetCharacterMovement) 0.0)
      (Animation|PlayAnimMontage "/Game/Models/Spider/Spider_Anim_Attack_Montage.Spider_Anim_Attack_Montage" 1.0 "None")
      (Utilities|FlowControl|Delay 1.0)
      (Game|SpawnActorfromClass "/Game/Enemies/Spiders/Spider/BP_Acid_Shoot.BP_Acid_Shoot_C" (Transformation|GetWorldTransform (Variables|Default|GetDirection)) "AdjustIfPossibleButAlwaysSpawn" "MultiplyWithRoot" 0 0)
      (AI|AIMoveTo _playerref "0, 0, 0" _playerref 5.0 false))
    (else
      (Variables|Default|SetAttacking? false))))

(event Game|Damage|EventAnyDamage
  (params (Damage :type Float%20%28single-precision%29) (DamageType :type Damage%20Type%20Object%20Reference) (InstigatedBy :type Controller%20Object%20Reference) (DamageCauser :type Actor%20Object%20Reference))
  ;[0.15 0.15 0.15 0.5] Getting hit
  (Utilities|Casting|CastToBP_PlayerAttackMelee DamageType
    (:then
      _)
    (:CastFailed
      (Utilities|Casting|CastToBP_PlayerAttackProjectail DamageType)))
  (Variables|Default|SetHP (- (Variables|Default|GetHP) Damage)))

(event EventTick
  (params (DeltaSeconds :type Float%20%28single-precision%29))
  (bind _healthbar (Variables|Default|GetHealthBar))
  ;[0.15 0.15 0.15 0.5] Event tick
  (if (> (Variables|Default|GetHP) 0.0)
    (bind _aswb_health_bar (Utilities|Casting|CastToWB_HealthBar (UserInterface|GetWidget (Variables|Default|GetHealthBar))))
    (Progress|SetPercent (Variables|/Game/UEStaff/Characters/WB_HealthBar.WB_HealthBar_C|GetHpBar _aswb_health_bar) (/ (Variables|Default|GetHP) 8e+01))
    (Transformation|SetWorldRotation _healthbar (Math|Rotator|FindLookatRotation (Transformation|GetWorldLocation _healthbar) (Transformation|GetWorldLocation (Variables|/Script/Engine.Actor|GetRootComponent (Game|GetPlayerCameraManager 0)))) false false)
    (if (Variables|Default|GetSeePlayer?)
      (CallFunction|Shoot)
      (else
        (Variables|Default|SetAttacking? false)))
    (else
      (Actor|DestroyActor))))

(event EventBeginPlay
  ;[0.15 0.15 0.15 0.5] Begin play
  (bind _asbp_third_person_character (Utilities|Casting|CastToBP_ThirdPersonCharacter (Game|GetPlayerCharacter 0)))
  (Variables|Default|SetPlayerRef _asbp_third_person_character)
  (CallFunction|StartRoam))

(fn ConstructionScript)