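; Tank spider enemy that roams the navmesh, chases the player inside its detection sphere, and attacks on sight.
; Pawn sensing triggers a montage and short forward sphere trace for damage, then a retreat to a random point behind it, re-rolled until the path is short enough.
; Only player melee and projectile damage types reduce HP.
; Tick updates the camera-facing health bar and handles death by playing a sound and destroying the actor.
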(event OnSeePawn(PawnSensing)
  (params (Pawn :type Pawn%20Object%20Reference))
  (bind _charactermovement (Variables|Character|GetCharacterMovement))
  (bind _playerref (Variables|Default|GetPlayerRef))
  ;[0.15 0.15 0.15 0.5] Attack
  (if (not (Variables|Default|GetAttacking?))
    (Variables|Default|SetAttacking? true)
    (Variables|/Script/Engine.CharacterMovementComponent|SetMaxWalkSpeed _charactermovement 0.0)
    (Animation|PlayAnimMontage "/Game/Models/Spider/Spider_Anim_Attack_Montage.Spider_Anim_Attack_Montage" 1.0 "None")
    (Utilities|FlowControl|Delay 0.2)
    (bind (_outhit _returnvalue) (Collision|SphereTraceForObjects (Transformation|GetActorLocation) (+ (Transformation|GetActorLocation) (* (Transformation|GetActorForwardVector) 7e+01)) 3e+01 (Utilities|Array|MakeArray "ObjectTypeQuery3") false 0 "None"))
    (if _returnvalue
      (if (== (.HitActor (Collision|BreakHitResult _outhit)) _playerref)
        (Game|Damage|ApplyDamage _playerref (Variables|Default|GetDemage) 0 0 "/Game/Blueprinty_silnika/BP_EnemyAttack.BP_EnemyAttack_C")))
    (Utilities|FlowControl|Delay 0.2)
    (Variables|/Script/Engine.CharacterMovementComponent|SetMaxWalkSpeed _charactermovement 6e+02)
    (bind _randomlocation (Class|NavigationSystemV1|GetRandomLocationinNavigableRadius (+ (Transformation|GetActorLocation) (* (Transformation|GetActorForwardVector) -8e+02)) 7e+02 0 0 :!label _label))
    (bind _returnvalue_2 (Class|NavigationSystemV1|FindPathtoLocationSynchronously (Transformation|GetActorLocation) _randomlocation 0 0))
    (if (< (Class|NavigationPath|GetPathLength _returnvalue_2) 1e+03)
      (AI|AIMoveTo self _randomlocation 0 5.0 false
        (:OnSuccess
          _)
        (:OnFail
          _))
      (Variables|Default|SetAttacking? false)
      (CallFunction|StartRoam)
      (else
        (goto _label)))))

(event OnComponentBeginOverlap(Sphere)
  (params (OverlappedComponent :type Primitive%20Component%20Object%20Reference) (OtherActor :type Actor%20Object%20Reference) (OtherComp :type Primitive%20Component%20Object%20Reference) (OtherBodyIndex :type Integer) (bFromSweep :type Boolean) (SweepResult :type Hit%20Result%20Structure%20%28by%20ref%29))
  ;[0.15 0.15 0.15 0.5] Saw player
  (if (== OtherActor (Variables|Default|GetPlayerRef))
    (Variables|Default|SetSeePlayer? true)
    (CallFunction|StartRoam)))

(event OnComponentEndOverlap(Sphere)
  (params (OverlappedComponent :type Primitive%20Component%20Object%20Reference) (OtherActor :type Actor%20Object%20Reference) (OtherComp :type Primitive%20Component%20Object%20Reference) (OtherBodyIndex :type Integer))
  ;[0.15 0.15 0.15 0.5] Saw player
  (if (== (Variables|Default|GetPlayerRef) OtherActor)
    (Variables|Default|SetSeePlayer? false)
    (CallFunction|StartRoam)))

(event Custom|Start%20Roam
  (bind _self self)
  (bind _charactermovement (Variables|Character|GetCharacterMovement))
  ;[0.15 0.15 0.15 0.5] Roaming, and follow player
  (if (not (Variables|Default|GetAttacking?))
    (if (Variables|Default|GetSeePlayer?)
      (Variables|/Script/Engine.CharacterMovementComponent|SetMaxWalkSpeed _charactermovement (Variables|Default|GetRunSpeed))
      (AI|AIMoveTo _self "0, 0, 0" (Variables|Default|GetPlayerRef) 5.0 false
        (:OnSuccess
          _)
        (:OnFail
          _))
      (else
        (Variables|/Script/Engine.CharacterMovementComponent|SetMaxWalkSpeed _charactermovement (Variables|Default|GetWalkSpeed))
        (bind _randomlocation (Class|NavigationSystemV1|GetRandomLocationinNavigableRadius (Transformation|GetActorLocation) (Variables|Default|GetRoamRadius) 0 0))
        (AI|AIMoveTo _self _randomlocation 0 5.0 false
          (:OnSuccess
            _)
          (:OnFail
            _))))
    (CallFunction|StartRoam)))

(event Game|Damage|EventAnyDamage
  (params (Damage :type Float%20%28single-precision%29) (DamageType :type Damage%20Type%20Object%20Reference) (InstigatedBy :type Controller%20Object%20Reference) (DamageCauser :type Actor%20Object%20Reference))
  ;[0.15 0.15 0.15 0.5] Getting hit
  (Utilities|Casting|CastToBP_PlayerAttackMelee DamageType
    (:then
      _)
    (:CastFailed
      (Utilities|Casting|CastToBP_PlayerAttackProjectail DamageType)))
  (Variables|Default|SetHP (- (Variables|Default|GetHP) Damage)))

(event EventTick
  (params (DeltaSeconds :type Float%20%28single-precision%29))
  (bind _healthbar (Variables|Default|GetHealthBar))
  ;[0.15 0.15 0.15 0.5] Event tick
  (if (> (Variables|Default|GetHP) 0.0)
    (bind _aswb_health_bar (Utilities|Casting|CastToWB_HealthBar (UserInterface|GetWidget (Variables|Default|GetHealthBar))))
    (Progress|SetPercent (Variables|/Game/UEStaff/Characters/WB_HealthBar.WB_HealthBar_C|GetHpBar _aswb_health_bar) (/ (Variables|Default|GetHP) 2e+02))
    (Transformation|SetWorldRotation _healthbar (Math|Rotator|FindLookatRotation (Transformation|GetWorldLocation _healthbar) (Transformation|GetWorldLocation (Variables|/Script/Engine.Actor|GetRootComponent (Game|GetPlayerCameraManager 0)))) false false)
    (else
      (Audio|PlaySoundatLocation "/Game/SFX/pająk_dead.pająk_dead" (Transformation|GetWorldLocation (Variables|Collision|GetCapsuleComponent)) "0, 0, 0" 1.0 1.0 0.0 0 0 0 0)
      (Actor|DestroyActor))))

(event EventBeginPlay
  ;[0.15 0.15 0.15 0.5] Begin play
  (bind _asbp_third_person_character (Utilities|Casting|CastToBP_ThirdPersonCharacter (Game|GetPlayerCharacter 0)))
  (Variables|Default|SetPlayerRef _asbp_third_person_character)
  (CallFunction|StartRoam))

(fn ConstructionScript)