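; Acid projectile from the spider enemy that damages pawns it touches and leaves an acid puddle on the ground.
; On bounce, it spawns BP_DropFloorAcid at the fluid component's location, aligned to the impact normal, then destroys itself.
; On sphere overlap, a small sphere trace finds a pawn and applies BP_EnemyAttack damage.
; The projectile is destroyed after that hit only if the pawn is the player character.
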(event OnProjectileBounce(Projetal)
  (params (ImpactResult :type Hit%20Result%20Structure%20%28by%20ref%29) (ImpactVelocity :type Vector%20%28by%20ref%29 :default "0, 0, 0"))
  ;[0.15 0.15 0.15 0.5] Usuwanie pocisku jak upadnie na ziemie + tworzenie małego jeziorka kwasu
  (Game|SpawnActorfromClass "/Game/Enemies/Bosses/Spider_boss/Blueprints/BP_DropFloorAcid.BP_DropFloorAcid_C" (Math|Transform|MakeTransform (Transformation|GetWorldLocation (Variables|Default|GetFluid_0)) (Math|Rotator|MakeRotfromZ (.ImpactNormal (Collision|BreakHitResult ImpactResult)))) "AdjustIfPossibleButAlwaysSpawn" "MultiplyWithRoot" 0 0)
  (Actor|DestroyActor))

(event OnComponentBeginOverlap(Sphere)
  (params (OverlappedComponent :type Primitive%20Component%20Object%20Reference) (OtherActor :type Actor%20Object%20Reference) (OtherComp :type Primitive%20Component%20Object%20Reference) (OtherBodyIndex :type Integer) (bFromSweep :type Boolean) (SweepResult :type Hit%20Result%20Structure%20%28by%20ref%29))
  (bind _returnvalue (Transformation|GetActorLocation))
  ;[0.15 0.15 0.15 0.5] GotHit (aktualnie ma nie zadawać demage)
  (bind (_outhit _returnvalue_2) (Collision|SphereTraceForObjects _returnvalue _returnvalue 3e+01 (Utilities|Array|MakeArray "ObjectTypeQuery3") false 0 "None"))
  (if _returnvalue_2
    (Game|Damage|ApplyDamage (.HitActor (Collision|BreakHitResult _outhit)) (Variables|Default|GetDamage) 0 0 "/Game/Blueprinty_silnika/BP_EnemyAttack.BP_EnemyAttack_C")
    (Utilities|Casting|CastToBP_ThirdPersonCharacter (.HitActor (Collision|BreakHitResult _outhit)))
    (Actor|DestroyActor)))

(fn ConstructionScript)