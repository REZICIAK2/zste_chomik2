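; BP_DropsOfAcid is an acid drop projectile for the Spider boss that leaves a small acid pool where it lands.
; When the projectile movement bounces, it spawns BP_DropFloorAcid at the Fluid0 component's location and destroys itself.
; The drop deals no direct damage: the sphere overlap event is empty, and the sphere-trace damage logic against pawns is disconnected.
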(event OnProjectileBounce(Projetal)
  (params (ImpactResult :type Hit%20Result%20Structure%20%28by%20ref%29) (ImpactVelocity :type Vector%20%28by%20ref%29 :default "0, 0, 0"))
  ;[0.15 0.15 0.15 0.5] Usuwanie pocisku jak upadnie na ziemie + tworzenie małego jeziorka kwasu
  (Game|SpawnActorfromClass "/Game/Enemies/Bosses/Spider_boss/Blueprints/BP_DropFloorAcid.BP_DropFloorAcid_C" (Math|Conversions|ToTransform(Vector) (Transformation|GetWorldLocation (Variables|Default|GetFluid_0))) "AdjustIfPossibleButAlwaysSpawn" "MultiplyWithRoot" 0 0)
  (Actor|DestroyActor))

(event OnComponentBeginOverlap(Sphere)
  (params (OverlappedComponent :type Primitive%20Component%20Object%20Reference) (OtherActor :type Actor%20Object%20Reference) (OtherComp :type Primitive%20Component%20Object%20Reference) (OtherBodyIndex :type Integer) (bFromSweep :type Boolean) (SweepResult :type Hit%20Result%20Structure%20%28by%20ref%29))
  ;[0.15 0.15 0.15 0.5] GotHit (aktualnie ma nie zadawać demage)
)

(fn ConstructionScript)