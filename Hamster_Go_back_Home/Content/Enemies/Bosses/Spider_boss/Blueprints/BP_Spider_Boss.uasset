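; Spider boss that fights the player in phases, with a health bar that faces the camera.
; It fires repeating acid projectiles at players inside its sphere, retreating at two health thresholds to spawn spider waves.
; Minions attach to a helper actor, whose attached count blocks boss damage and signals wave end.
; After the second wave it chases and melees via pawn sensing, while Tick yaws the body to follow its head socket.
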(event OnSeePawn(PawnSensing)
  (params (Pawn :type Pawn%20Object%20Reference))
  (bind _playerref (Variables|Default|GetPlayerRef))
  ;[0.15 0.15 0.15 0.5] Meele attack
  (if (and (Variables|Default|GetCanAttack?) (Variables|Default|GetIsLastPhase))
    (Variables|Default|SetCanAttack? false)
    (CallFunction|ChangeMaxWalkSpeed 0.0)
    (Animation|PlayAnimMontage "/Game/Models/Spider/Spider_Attack_Montage.Spider_Attack_Montage" 1.0 "None")
    (Utilities|FlowControl|Delay 0.2)
    (bind (_outhit _returnvalue) (Collision|SphereTraceForObjects (Transformation|GetActorLocation) (+ (Transformation|GetActorLocation) (* (Transformation|GetActorForwardVector) 1e+02)) 5e+01 (Utilities|Array|MakeArray "ObjectTypeQuery3") false 0 "None"))
    (if _returnvalue
      (if (== (.HitActor (Collision|BreakHitResult _outhit)) _playerref)
        (Game|Damage|ApplyDamage _playerref (Variables|Default|GetDemage) 0 0 "/Game/Blueprinty_silnika/BP_EnemyAttack.BP_EnemyAttack_C" :!label _label)
        (Utilities|FlowControl|Delay 1.0)
        (CallFunction|ChangeMaxWalkSpeed 5e+02)
        (Utilities|FlowControl|Delay 2.0)
        (Variables|Default|SetCanAttack? true))
      (else
        (goto _label)))))

(event OnComponentBeginOverlap(Sphere)
  (params (OverlappedComponent :type Primitive%20Component%20Object%20Reference) (OtherActor :type Actor%20Object%20Reference) (OtherComp :type Primitive%20Component%20Object%20Reference) (OtherBodyIndex :type Integer) (bFromSweep :type Boolean) (SweepResult :type Hit%20Result%20Structure%20%28by%20ref%29))
  ;[0.15 0.15 0.15 0.5] Saw player
  (if (== OtherActor (Variables|Default|GetPlayerRef))
    (Variables|Default|SetSeePlayer? true)
    (CallFunction|AcidAttack)))

(event OnComponentEndOverlap(Sphere)
  (params (OverlappedComponent :type Primitive%20Component%20Object%20Reference) (OtherActor :type Actor%20Object%20Reference) (OtherComp :type Primitive%20Component%20Object%20Reference) (OtherBodyIndex :type Integer))
  ;[0.15 0.15 0.15 0.5] Saw player
  (if (== (Variables|Default|GetPlayerRef) OtherActor)
    (Variables|Default|SetSeePlayer? false)))

(event Custom|AcidAttack
  (bind _mesh (Variables|Character|GetMesh))
  (bind _projectail_spawn (Variables|Default|GetProjectail%20Spawn))
  (bind _returnvalue (Transformation|GetSocketRotation _mesh "head"))
  ;[0.15 0.15 0.15 0.5] Shoot player
  (if (Math|Boolean|ANDBoolean (not (Variables|Default|GetIsLastPhase)) (not (Variables|Default|GetIsWave)) (Variables|Default|GetSeePlayer?) (Variables|Default|GetCanAttack?))
    (Variables|Default|SetCanAttack? false)
    (Transformation|SetWorldRotation _projectail_spawn (Math|Rotator|MakeRotator (.roll _returnvalue) 1e+01 (+ (.yaw _returnvalue) -9e+01)) false false)
    (Game|SpawnActorfromClass "/Game/Enemies/Bosses/Spider_boss/Blueprints/BP_AcidProjectail.BP_AcidProjectail_C" (Transformation|GetWorldTransform _projectail_spawn) "AlwaysSpawn" "MultiplyWithRoot" 0 0)
    (Utilities|FlowControl|Delay 3.0)
    (Variables|Default|SetCanAttack? true)
    (CallFunction|AcidAttack)))

(event Custom|StartWave
  (params (NumberOfEnemies :type Integer))
  ;[0.15 0.15 0.15 0.5] First WaveThreshold
  (for _index (range 1 NumberOfEnemies)
    (bind _randomlocation (Class|NavigationSystemV1|GetRandomLocationinNavigableRadius (Variables|Default|GetStartLocation) 5e+02 0 0))
    (bind _returnvalue (Game|SpawnActorfromClass "/Game/Enemies/Spider/Blueprints/BP_Spider.BP_Spider_C" (Math|Transform|MakeTransform _randomlocation "0, 0, 0" "1.000000,1.000000,1.000000") "AdjustIfPossibleButAlwaysSpawn" "MultiplyWithRoot" 0 0))
    (Transformation|AttachActorToActor _returnvalue (Variables|Default|GetSpidersParent) "None" "KeepWorld" "KeepWorld" "KeepWorld" true)))

(event Custom|RotateToPlayer
  (bind _mesh (Variables|Character|GetMesh))
  (bind _capsulecomponent (Variables|Collision|GetCapsuleComponent))
  (bind _returnvalue (Transformation|GetSocketRotation _mesh "head"))
  (bind _returnvalue_2 (Transformation|GetWorldRotation _mesh))
  (bind _returnvalue_3 (Transformation|GetWorldRotation _capsulecomponent))
  (bind _returnvalue_4 (Math|Rotator|Delta(Rotator) (Math|Rotator|MakeRotator 0.0 0.0 (.yaw _returnvalue)) (Math|Rotator|MakeRotator 0.0 0.0 (.yaw _returnvalue_2))))
  (bind _returnvalue_5 (< (.roll _returnvalue) -3e+01))
  ;[0.15 0.15 0.15 0.5] Rotate to player
  (if (or (> (.yaw _returnvalue_4) 35.0) (and _returnvalue_5 (> (.yaw _returnvalue_4) 1.0)))
    (Variables|Default|SetRotationToPlayer (+ (.yaw _returnvalue_3) 0.5))
    (Transformation|SetWorldRotation (Variables|Collision|GetCapsuleComponent) (Math|Rotator|MakeRotator (.roll _returnvalue_3) (.pitch _returnvalue_3) (Variables|Default|GetRotationToPlayer)) false false :!label _label)
    (elif (or (< (.yaw _returnvalue_4) -35.0) (and _returnvalue_5 (< (.yaw _returnvalue_4) -1.0)))
      (Variables|Default|SetRotationToPlayer (- (.yaw _returnvalue_3) 0.5))
      (goto _label))))

(event Custom|StalkPlayer
  ;[0.15 0.15 0.15 0.5] Stalking player
  (Variables|/Script/Engine.CharacterMovementComponent|SetMaxWalkSpeed (Variables|Character|GetCharacterMovement) 5e+02)
  (AI|AIMoveTo self "0, 0, 0" (Game|GetPlayerCharacter 0) 5.0 false
    (:OnSuccess
      _)
    (:OnFail
      _))
  (CallFunction|StalkPlayer))

(event Custom|ChangeMaxWalkSpeed
  (params (Walk%20Speed :type Float%20%28double-precision%29))
  ;[0.15 0.15 0.15 0.5] Function to change speed
  (Variables|/Script/Engine.CharacterMovementComponent|SetMaxWalkSpeed (Variables|Character|GetCharacterMovement) Walk%20Speed))

(event Game|Damage|EventAnyDamage
  (params (Damage :type Float%20%28single-precision%29) (DamageType :type Damage%20Type%20Object%20Reference) (InstigatedBy :type Controller%20Object%20Reference) (DamageCauser :type Actor%20Object%20Reference))
  ;[0.15 0.15 0.15 0.5] Getting hit
  (Utilities|Casting|CastToBP_PlayerAttackMelee DamageType
    (:then
      _)
    (:CastFailed
      (Utilities|Casting|CastToBP_PlayerAttackProjectail DamageType)))
  (if (== (Utilities|Array|Length (Actor|GetAttachedActors (Variables|Default|GetSpidersParent) true false)) 0)
    (Variables|Default|SetHP (- (Variables|Default|GetHP) Damage))))

(event EventTick
  (params (DeltaSeconds :type Float%20%28single-precision%29))
  (bind _self self)
  (bind _healthbar (Variables|Components|GetHealthBar))
  ;[0.15 0.15 0.15 0.5] Event tick
  (CallFunction|RotatetoPlayer)
  (if (> (Variables|Default|GetHP) 0.0)
    (bind _aswb_health_bar (Utilities|Casting|CastToWB_HealthBar (UserInterface|GetWidget (Variables|Components|GetHealthBar))))
    (Progress|SetPercent (Variables|/Game/Characters/WB_HealthBar.WB_HealthBar_C|GetHpBar _aswb_health_bar) (/ (Variables|Default|GetHP) (Variables|Default|GetMaxHP)))
    (Transformation|SetWorldRotation _healthbar (Math|Rotator|FindLookatRotation (Transformation|GetWorldLocation _healthbar) (Transformation|GetWorldLocation (Variables|/Script/Engine.Actor|GetRootComponent (Game|GetPlayerCameraManager 0)))) false false)
    (if (and (Variables|Default|GetIsWave) (== (Utilities|Array|Length (Actor|GetAttachedActors (Variables|Default|GetSpidersParent) true false)) 0))
      (Utilities|FlowControl|FlipFlop
        (:A
          (Variables|Default|SetIsWave false)
          (AI|AIMoveTo self (Variables|Default|GetStartLocation) 0 2.0 false
            (:OnSuccess
              _)
            (:OnFail
              _))
          (Utilities|FlowControl|Delay 3.0)
          (Variables|Default|SetCanAttack? true)
          (if (not (Variables|Default|GetSeePlayer?))
            (CallFunction|AcidAttack)))
        (:B
          (Variables|Default|SetIsLastPhase true)
          (Variables|Default|SetIsWave false)
          (CallFunction|StalkPlayer)))
      (elif (< (Variables|Default|GetHP) (Variables|Default|GetWaveThreshold))
        (Variables|Default|SetIsWave true)
        (Utilities|FlowControl|FlipFlop
          (:A
            (Variables|Default|SetHP (Variables|Default|GetWaveThreshold))
            (Variables|Default|SetWaveThreshold (* (Variables|Default|GetMaxHP) 0.333))
            (Variables|Default|SetCanAttack? false)
            (CallFunction|StartWave 1)
            (AI|AIMoveTo _self (+ (Variables|Default|GetStartLocation) "-1000.000000,0.000000,0.000000") 0 5.0 false))
          (:B
            (Variables|Default|SetWaveThreshold -1.0)
            (Variables|Default|SetCanAttack? false)
            (CallFunction|StartWave 1)
            (AI|AIMoveTo _self (+ (Variables|Default|GetStartLocation) "1000.000000,0.000000,0.000000") 0 5.0 false)))))
    (else
      (Actor|DestroyActor))))

(event EventBeginPlay
  ;[0.15 0.15 0.15 0.5] Begin play
  (Variables|Default|SetWaveThreshold (* (Variables|Default|GetHP) 0.666))
  (bind _asbp_third_person_character (Utilities|Casting|CastToBP_ThirdPersonCharacter (Game|GetPlayerCharacter 0)))
  (Variables|Default|SetPlayerRef _asbp_third_person_character)
  (Variables|Default|SetStartLocation (Transformation|GetActorLocation))
  (bind _returnvalue (Game|SpawnActorfromClass "/Game/Enemies/Bosses/Spider_boss/Blueprints/BP_Boss_Spiders_Parent.BP_Boss_Spiders_Parent_C" (Math|Transform|MakeTransform "0, 0, 0" "0, 0, 0" "1.000000,1.000000,1.000000") "AlwaysSpawn" "MultiplyWithRoot" 0 0))
  (Variables|Default|SetSpidersParent _returnvalue)
  (CallFunction|ChangeMaxWalkSpeed 5e+02))

(fn ConstructionScript)