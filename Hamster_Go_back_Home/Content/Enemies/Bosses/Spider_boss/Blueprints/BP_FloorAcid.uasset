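; Spider boss acid pool that applies damage over time to the player standing in it and removes itself after about five seconds.
; On BeginPlay it picks a random splat mesh and spawns several acid drops at random angles.
; Capsule overlaps adjust a pool counter on the player, so the DOT is switched off only after leaving the last pool.
; Timelines scale the bubble and then the pool before the actor is destroyed.
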(event OnComponentBeginOverlap(Capsule)
  (params (OverlappedComponent :type Primitive%20Component%20Object%20Reference) (OtherActor :type Actor%20Object%20Reference) (OtherComp :type Primitive%20Component%20Object%20Reference) (OtherBodyIndex :type Integer) (bFromSweep :type Boolean) (SweepResult :type Hit%20Result%20Structure%20%28by%20ref%29))
  (bind _as_bp_third_person_character (Variables|Default|GetAs%20BP%20Third%20Person%20Character))
  ;[0.15 0.15 0.15 0.5] DOT demage for player
  (if (== OtherActor _as_bp_third_person_character)
    (Variables|/Game/ThirdPerson/Blueprints/BP_ThirdPersonCharacter.BP_ThirdPersonCharacter_C|SetAcidPoolsCounter _as_bp_third_person_character (+ (Variables|/Game/ThirdPerson/Blueprints/BP_ThirdPersonCharacter.BP_ThirdPersonCharacter_C|GetAcidPoolsCounter _as_bp_third_person_character) 1.0))
    (Default|ApplyAcidDOT _as_bp_third_person_character true 1.0 1.0)))

(event OnComponentEndOverlap(Capsule)
  (params (OverlappedComponent :type Primitive%20Component%20Object%20Reference) (OtherActor :type Actor%20Object%20Reference) (OtherComp :type Primitive%20Component%20Object%20Reference) (OtherBodyIndex :type Integer))
  (bind _as_bp_third_person_character (Variables|Default|GetAs%20BP%20Third%20Person%20Character))
  ;[0.15 0.15 0.15 0.5] DOT demage for player
  (if (== OtherActor _as_bp_third_person_character)
    (Variables|/Game/ThirdPerson/Blueprints/BP_ThirdPersonCharacter.BP_ThirdPersonCharacter_C|SetAcidPoolsCounter _as_bp_third_person_character (- (Variables|/Game/ThirdPerson/Blueprints/BP_ThirdPersonCharacter.BP_ThirdPersonCharacter_C|GetAcidPoolsCounter _as_bp_third_person_character) 1.0))
    (if (== (Variables|/Game/ThirdPerson/Blueprints/BP_ThirdPersonCharacter.BP_ThirdPersonCharacter_C|GetAcidPoolsCounter _as_bp_third_person_character) 0.0)
      (Default|ApplyAcidDOT _as_bp_third_person_character false 1.0 1.0))))

(event Custom|mesh%20change
  ;[0.15 0.15 0.15 0.5] Podmiana Static mesh
  (Components|StaticMesh|SetStaticMesh (Variables|Default|Getacidd) (.OutItem (Utilities|Array|Random (Variables|Default|GetPlama)))))

(event Custom|acid
  ;[0.15 0.15 0.15 0.5] tworzenie jeziorka kwasu
  (Transformation|SetWorldRotation (Variables|Default|GetArrow) (Math|Rotator|MakeRotator 0.0 (Math|Random|RandomFloatinRange 3e+01 1.5e+02) (Math|Random|RandomFloatinRange 0.0 3.6e+02)) false false)
  (Game|SpawnActorfromClass "/Game/Enemies/Bosses/Spider_boss/Blueprints/BP_DropsOfAcid.BP_DropsOfAcid_C" (Transformation|GetWorldTransform (Variables|Default|GetArrow)) "AdjustIfPossibleButAlwaysSpawn" "MultiplyWithRoot" 0 0))

(event Custom|destroyanim
  (params (Delate :type Boolean))
  ;[0.15 0.15 0.15 0.5] usuwanie kwasu
  (if Delate
    (bind _newtrack_0 (Timeline|Timeline PlayFromStart)
      (:Update
        (Transformation|SetRelativeScale3D (Variables|Default|Getacidd) (Math|Vector|MakeVector _newtrack_0 _newtrack_0 (/ _newtrack_0 1e+01))))
      (:Finished
        (Actor|DestroyActor)))
    (else
      (bind _newtrack_0_2 (Timeline|Timeline_0 PlayFromStart)
        (:Update
          (Transformation|SetRelativeScale3D (Variables|Default|Getbuble) (Math|Vector|MakeVector (* _newtrack_0_2 0.1) (* _newtrack_0_2 0.1) (* (/ _newtrack_0_2 1e+01) 0.1))))
        (:Finished
          (Rendering|SetVisibility (Variables|Default|Getbuble) false false))))))

(event EventBeginPlay
  ;[0.15 0.15 0.15 0.5] tworzenie kropel kwasu
  (CallFunction|MeshChange)
  (for _index (range 0 3)
    (CallFunction|Acid)
    (bind _asbp_third_person_character (Utilities|Casting|CastToBP_ThirdPersonCharacter (Game|GetPlayerCharacter 0)))
    (Variables|Default|SetAs%20BP%20Third%20Person%20Character _asbp_third_person_character))
  (Utilities|FlowControl|Delay 4.8)
  (CallFunction|Destroyanim false)
  (Utilities|FlowControl|Delay 0.2)
  (CallFunction|Destroyanim true))

(fn ConstructionScript)