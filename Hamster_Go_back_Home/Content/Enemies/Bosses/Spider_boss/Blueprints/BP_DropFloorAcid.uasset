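; Acid pool actor in the spider boss assets that applies damage over time to the player standing in it.
; On spawn it picks a random splat mesh, waits briefly, then a timeline scales it with a flattened Z before the actor is destroyed.
; Sphere overlaps adjust a pool counter on the player, so damage stops when the count reaches zero.
; Timeline completion also switches the damage off, regardless of that counter.
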(event OnComponentBeginOverlap(Sphere)
  (params (OverlappedComponent :type Primitive%20Component%20Object%20Reference) (OtherActor :type Actor%20Object%20Reference) (OtherComp :type Primitive%20Component%20Object%20Reference) (OtherBodyIndex :type Integer) (bFromSweep :type Boolean) (SweepResult :type Hit%20Result%20Structure%20%28by%20ref%29))
  (bind _as_bp_third_person_character (Variables|Default|GetAs%20BP%20Third%20Person%20Character))
  ;[0.15 0.15 0.15 0.5] DOT demage for player
  (if (== OtherActor _as_bp_third_person_character)
    (Variables|/Game/ThirdPerson/Blueprints/BP_ThirdPersonCharacter.BP_ThirdPersonCharacter_C|SetAcidPoolsCounter _as_bp_third_person_character (+ (Variables|/Game/ThirdPerson/Blueprints/BP_ThirdPersonCharacter.BP_ThirdPersonCharacter_C|GetAcidPoolsCounter _as_bp_third_person_character) 1.0))
    (Default|ApplyAcidDOT _as_bp_third_person_character true 1.0 1.0)))

(event OnComponentEndOverlap(Sphere)
  (params (OverlappedComponent :type Primitive%20Component%20Object%20Reference) (OtherActor :type Actor%20Object%20Reference) (OtherComp :type Primitive%20Component%20Object%20Reference) (OtherBodyIndex :type Integer))
  (bind _as_bp_third_person_character (Variables|Default|GetAs%20BP%20Third%20Person%20Character))
  ;[0.15 0.15 0.15 0.5] DOT demage for player
  (if (== OtherActor _as_bp_third_person_character)
    (Variables|/Game/ThirdPerson/Blueprints/BP_ThirdPersonCharacter.BP_ThirdPersonCharacter_C|SetAcidPoolsCounter _as_bp_third_person_character (- (Variables|/Game/ThirdPerson/Blueprints/BP_ThirdPersonCharacter.BP_ThirdPersonCharacter_C|GetAcidPoolsCounter _as_bp_third_person_character) 1.0))
    (if (== (Variables|/Game/ThirdPerson/Blueprints/BP_ThirdPersonCharacter.BP_ThirdPersonCharacter_C|GetAcidPoolsCounter _as_bp_third_person_character) 0.0)
      (Default|ApplyAcidDOT _as_bp_third_person_character false 1.0 1.0))))

(event Custom|mesh%20change
  ;[0.15 0.15 0.15 0.5] Podmiana Static mesh
  (Components|StaticMesh|SetStaticMesh (Variables|Default|Getacid%20) (.OutItem (Utilities|Array|Random (Variables|Default|Getplama)))))

(event EventBeginPlay
  ;[0.15 0.15 0.15 0.5] usuwanie kwasu
  (bind _asbp_third_person_character (Utilities|Casting|CastToBP_ThirdPersonCharacter (Game|GetPlayerCharacter 0)))
  (Variables|Default|SetAs%20BP%20Third%20Person%20Character _asbp_third_person_character)
  (CallFunction|MeshChange)
  (Utilities|FlowControl|Delay 2.0)
  (bind _newtrack_0 (Timeline|Timeline Play)
    (:Update
      (Transformation|SetRelativeScale3D (Variables|Default|Getacid%20) (Math|Vector|MakeVector _newtrack_0 _newtrack_0 (/ _newtrack_0 1e+01))))
    (:Finished
      (Actor|DestroyActor)
      (Default|ApplyAcidDOT (Variables|Default|GetAs%20BP%20Third%20Person%20Character) false 0.0 0.0))))

(fn ConstructionScript)